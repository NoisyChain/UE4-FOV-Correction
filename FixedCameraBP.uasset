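; Shared camera actor that frames two players, Player1 and Player2, in a single view.
; On BeginPlay it creates and possesses a second local player, then becomes player 0's view target.
; Each tick it moves to the players' midpoint, clamped between walls on Y and raised by a height offset.
; The spring arm length scales with the distance between players within set limits, zooming as they separate.
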(event `self.ReceiveBeginPlay`
  (bind _returnvalue (`GameplayStatics.CreatePlayer` -1))
  (`Controller.Possess` _returnvalue null)
  (`PlayerController.SetViewTargetWithBlend` (`GameplayStatics.GetPlayerController` 0) self 0.0 "VTBlend_Linear" 0.0 false))

(event `self.ReceiveTick`
  (params (DeltaSeconds :type "Float (single-precision)"))
  (`self.K2_SetActorLocation` (`KismetMathLibrary.MakeVector` (.x (/ (+ (`self.K2_GetActorLocation` (`self.Player1`)) (`self.K2_GetActorLocation` (`self.Player2`))) 2.0)) (`KismetMathLibrary.FClamp` (.y (/ (+ (`self.K2_GetActorLocation` (`self.Player1`)) (`self.K2_GetActorLocation` (`self.Player2`))) 2.0)) (`self.MinimumWall`) (`self.MaximumWall`)) (+ (.z (/ (+ (`self.K2_GetActorLocation` (`self.Player1`)) (`self.K2_GetActorLocation` (`self.Player2`))) 2.0)) (`self.CameraHeight`))))
  (set `SpringArmComponent.TargetArmLength` (`KismetMathLibrary.FClamp` (* (`KismetMathLibrary.VSize` (- (`self.K2_GetActorLocation` (`self.Player2`)) (`self.K2_GetActorLocation` (`self.Player1`)))) 1.6) (`self.MinimumArmLength`) (`self.MaximumArmLength`)) (`self.SpringArm`)))

(fn `UserConstructionScript`)